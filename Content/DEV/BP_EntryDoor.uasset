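; BP_EntryDoor is a curse-aware double door that swings shut as the player approaches.
; While unfrozen and in range, Tick maps player distance within the Sphere to OpenPercentage, lerping both leaves' rotations.
; On character entry, the game state decides motion: a spelt, unlifted curse unfreezes the door and calls StartCurse, while a lifted curse freezes it.
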(event OnComponentBeginOverlap(Sphere)
  (params (OverlappedComponent :type Primitive%20Component%20Object%20Reference) (OtherActor :type Actor%20Object%20Reference) (OtherComp :type Primitive%20Component%20Object%20Reference) (OtherBodyIndex :type Integer) (bFromSweep :type Boolean) (SweepResult :type Hit%20Result%20Structure%20%28by%20ref%29))
  (bind _returnvalue (Game|GetGameState))
  (bind _asantrgame_state (Utilities|Casting|CastToANTRGameState _returnvalue))
  (bind _curselifted (Variables|/Game/ANTRGameState.ANTRGameState_C|GetCurseLifted _asantrgame_state))
  (Utilities|Casting|CastToANTRCharacter OtherActor)
  (Variables|Default|SetPlayerInRange true)
  (if (and (not _curselifted) (Variables|/Game/ANTRGameState.ANTRGameState_C|GetCurseSpelt _asantrgame_state))
    (Variables|Default|SetFrozen false)
    (Default|StartCurse (.AsANTRGame%20State (Utilities|Casting|CastToANTRGameState (Game|GetGameState))))
    (elif _curselifted
      (Variables|Default|SetFrozen true))))

(event OnComponentEndOverlap(Sphere)
  (params (OverlappedComponent :type Primitive%20Component%20Object%20Reference) (OtherActor :type Actor%20Object%20Reference) (OtherComp :type Primitive%20Component%20Object%20Reference) (OtherBodyIndex :type Integer))
  (Utilities|Casting|CastToANTRCharacter OtherActor)
  (Variables|Default|SetPlayerInRange false))

(event EventTick
  (params (DeltaSeconds :type Float%20%28single-precision%29))
  (if (not (Variables|Default|GetFrozen))
    (if (Variables|Default|GetPlayerInRange)
      (bind _output_get (Variables|Default|SetOpenPercentage (Math|Float|MapRangeClamped (Transformation|GetDistanceTo self (Game|GetPlayerCharacter 0)) 2e+02 (Variables|/Script/Engine.SphereComponent|GetSphereRadius (Variables|Default|GetSphere)) 0.0 1.0)))
      (Transformation|SetRelativeRotation (Variables|Default|GetLeftDoor) (Math|Rotator|Lerp(Rotator) "0,180.000000, 0" "0,-90.000000, 0" _output_get true) false false)
      (Transformation|SetRelativeRotation (Variables|Default|GetRightDoor) (Math|Rotator|Lerp(Rotator) "0, 0, 0" "0,-90.000000, 0" _output_get true) false false))))

(fn ConstructionScript)