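; BP_PickupBase is a base Blueprint for pickups that the NTR character collects by overlapping a sphere collider.
; The construction script sizes the collider from PickupRadius.
; On overlap by an ANTRCharacter it plays a pickup sound at its location, calls OnPickup and destroys itself.
; OnPickup is meant to be overridden in child Blueprints, and the base version only prints a red warning saying so.
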(event OnComponentBeginOverlap(Collider)
  (params (OverlappedComponent :type Primitive%20Component%20Object%20Reference) (OtherActor :type Actor%20Object%20Reference) (OtherComp :type Primitive%20Component%20Object%20Reference) (OtherBodyIndex :type Integer) (bFromSweep :type Boolean) (SweepResult :type Hit%20Result%20Structure%20%28by%20ref%29))
  (Utilities|Casting|CastToANTRCharacter OtherActor)
  (Audio|PlaySoundatLocation "/Game/Audio/SFX_Pickup.SFX_Pickup" (Transformation|GetActorLocation))
  (CallFunction|OnPickup)
  (Actor|DestroyActor))

(event EventBeginPlay)

(fn ConstructionScript
  (Components|Sphere|SetSphereRadius (Variables|Default|GetCollider) (Variables|Default|GetPickupRadius) false))

(fn OnPickup
  (Development|PrintString "Please Override OnPickup() functionality in inheriting blueprints!" true true "(R=1.000000,G=0.000000,B=0.000000,A=1.000000)" 6.0))