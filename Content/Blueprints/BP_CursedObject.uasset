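; BP_CursedObject is a pickup that lifts a curse when collected.
; Its OnPickup event prints an on-screen confirmation, then calls StopChase on every NTRCreeper actor in the level.
; The same loop sets CurseLifted on the NTRGameState, so the flag is only set when at least one creeper exists.
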(event EventBeginPlay
  (|CallParentFunction) ; This node is disabled and will not be called.\nDrag off pins to build functionality.
)

(event Collision|EventActorBeginOverlap
  (params (OtherActor :type Actor%20Object%20Reference)))

(event EventTick
  (params (DeltaSeconds :type Float%20%28single-precision%29)))

(event EventOnPickup
  (Development|PrintString "The Curse has been lifted" true true "(R=1.000000,G=0.500000,B=0.000000,A=1.000000)" 5.0)
  (bind _outactors (Actor|GetAllActorsOfClass "/Game/AI/ANTRCreeper.ANTRCreeper_C"))
  (for _array_element _outactors
    (Default|StopChase _array_element)
    (Variables|/Game/ANTRGameState.ANTRGameState_C|SetCurseLifted (.AsANTRGame%20State (Utilities|Casting|CastToANTRGameState (Game|GetGameState))) true)))

(fn ConstructionScript
  (|CallParentFunction))