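; Battery pickup Blueprint that credits the player with a battery when collected.
; Its OnPickup event increments Batteries on the first player's ANTRCharacter and BatteriesCollected on ANTRGameState, then prints a green confirmation message.
; BeginPlay and the construction script add no logic of their own.
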(event EventBeginPlay
  (|CallParentFunction) ; This node is disabled and will not be called.\nDrag off pins to build functionality.
)

(event EventOnPickup
  (Math|Integer|IncrementInt (Variables|/Game/Character/ANTRCharacter.ANTRCharacter_C|GetBatteries (.AsANTRCharacter (Utilities|Casting|CastToANTRCharacter (Game|GetPlayerCharacter 0))))
    (:%20%20
      (Math|Integer|IncrementInt (Variables|/Game/ANTRGameState.ANTRGameState_C|GetBatteriesCollected (.AsANTRGame%20State (Utilities|Casting|CastToANTRGameState (Game|GetGameState))))
        (:%20%20
          (Development|PrintString "Battery added" true true "(R=0.000000,G=1.000000,B=0.000000,A=1.000000)"))))))

(fn ConstructionScript
  (|CallParentFunction))